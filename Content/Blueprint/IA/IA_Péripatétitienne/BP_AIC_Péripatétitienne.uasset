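; AI controller for the Péripatétitienne NPC, driving it with its behavior tree.
; On begin play it runs BT_IA_Péripatétitienne, and on possess it casts the pawn to BP_IA_Péripatétitienne.
; A looping one-second timer then copies the pawn's chamber-assigned flag and chamber location into the blackboard, so the tree follows the pawn's state by polling.
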(event Custom|SetVariable
  (bind _returnvalue (AI|GetBlackboard 0))
  (AI|Components|Blackboard|SetValueasBool _returnvalue (Utilities|Name|MakeLiteralName "Chamber_Assigne") (Variables|/Game/Blueprint/IA/IA_Péripatétitienne/BP_IA_Péripatétitienne.BP_IA_Péripatétitienne_C|GetChamber? (stale EventPossess _asbp_ia_péripatétitienne)))
  (AI|Components|Blackboard|SetValueasVector _returnvalue (Utilities|Name|MakeLiteralName "ChamberPosition") (Variables|/Game/Blueprint/IA/IA_Péripatétitienne/BP_IA_Péripatétitienne.BP_IA_Péripatétitienne_C|GetChamber%20Location (stale EventPossess _asbp_ia_péripatétitienne))))

(event EventBeginPlay
  (AI|RunBehaviorTree "/Game/Blueprint/IA/IA_Péripatétitienne/BT_IA_Péripatétitienne.BT_IA_Péripatétitienne"))

(event EventPossess
  (params (PossessedPawn :type Pawn%20Object%20Reference))
  (bind _asbp_ia_péripatétitienne (Utilities|Casting|CastToBP_IA_Péripatétitienne PossessedPawn))
  (Utilities|Time|SetTimerbyEvent (delegate Custom|SetVariable) 1.0 true))

(fn ConstructionScript)